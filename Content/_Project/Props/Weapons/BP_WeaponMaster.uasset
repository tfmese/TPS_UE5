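; BP_WeaponMaster is a weapon Blueprint, apparently a base class by its name, that handles magazine ammo consumption for the player's weapon.
; On BeginPlay it caches the player's BP_ThirdPersonCharacter.
; TryFireAndConsumeAmmo decrements the clamped magazine count, sends magazine and reserve values to the character through CallEUpdateAmmo and returns true.
; With an empty magazine it tells the character to cease auto fire and returns false.
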(event `self.ReceiveBeginPlay`
  (bind _asbp_third_person_character (cast `/Game/ThirdPerson/Blueprints/BP_ThirdPersonCharacter` (`GameplayStatics.GetPlayerCharacter` 0)))
  (set `self.Player Character` _asbp_third_person_character))

(fn `TryFireAndConsumeAmmo`
  (returns (`CanFireAgain?` :type Boolean))
  (bind _returnvalue (`KismetMathLibrary.Clamp` (- (`self.CurrentMagAmmo`) 1) 0 (`self.MaxMagAmmo`)))
  (if (> (`self.CurrentMagAmmo`) 0)
    (bind _output_get (set `self.CurrentMagAmmo` _returnvalue))
    (`/Game/ThirdPerson/Blueprints/BP_ThirdPersonCharacter.E_UpdateAmmo` (`self.Player Character`) _returnvalue (`self.CurentReserveAmmo`))
    (return true)
    (else
      (`/Game/ThirdPerson/Blueprints/BP_ThirdPersonCharacter.Cease Auto Fire` (`self.Player Character`))
      (return false))))