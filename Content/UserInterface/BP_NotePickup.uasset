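; BP_NotePickup is an interactable note actor that lets the player open and read its text on screen.
; A sphere overlap with the third-person character shows a prompt Widget component and sets an in-range flag (OyuncuAlandaMı).
; Pressing E in range creates a WBP_NoteDisplay with NoteContent, adds it to the viewport, and switches to UI-only input with a visible mouse cursor.
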(event `Key|E`
  (params (Key :type "Key Structure"))
  (bind _returnvalue (`GameplayStatics.GetPlayerController` 0))
  (:`Pressed`
    (if (`self.OyuncuAlandaMı`)
      (bind _returnvalue_2 (`|CreateWidget` "/Game/UserInterface/WBP_NoteDisplay.WBP_NoteDisplay_C" null (`self.NoteContent`)))
      (`UserWidget.AddToViewport` _returnvalue_2 0)
      (`WidgetBlueprintLibrary.SetInputMode_UIOnlyEx` _returnvalue null)
      (set `PlayerController.bShowMouseCursor` true _returnvalue))))

(event `self.Sphere1.OnComponentBeginOverlap`
  (params (OverlappedComponent :type "PrimitiveComponent Object Reference") (OtherActor :type "Actor Object Reference") (OtherComp :type "PrimitiveComponent Object Reference") (OtherBodyIndex :type Integer) (bFromSweep :type Boolean) (SweepResult :type "HitResult Structure (by ref)"))
  (cast `/Game/ThirdPerson/Blueprints/BP_ThirdPersonCharacter` OtherActor)
  (`SceneComponent.SetVisibility` (`self.Widget`) true false)
  (set `self.OyuncuAlandaMı` true))

(event `self.Sphere1.OnComponentEndOverlap`
  (params (OverlappedComponent :type "PrimitiveComponent Object Reference") (OtherActor :type "Actor Object Reference") (OtherComp :type "PrimitiveComponent Object Reference") (OtherBodyIndex :type Integer))
  (cast `/Game/ThirdPerson/Blueprints/BP_ThirdPersonCharacter` OtherActor)
  (`SceneComponent.SetVisibility` (`self.Widget`) false false)
  (set `self.OyuncuAlandaMı` false))

(fn `UserConstructionScript`)