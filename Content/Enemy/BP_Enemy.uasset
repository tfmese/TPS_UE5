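; Enemy AI character that spawns with an attached weapon and reacts to perceiving the third-person player.
; BeginPlay seeds the Blackboard with a random walk speed, start location and patrol point.
; Perception updates set the target or last known location and show an alert widget, which Tick clears once the lost-target timer exceeds GiveUpTime.
; A ragdoll death handler exists, but the health component's death binding is never executed.
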(event `self.ReceiveBeginPlay`
  (bind _returnvalue (`|SpawnActorFromClass` "/Game/Enemy/BP_EnemyWeapon.BP_EnemyWeapon_C" (`self.GetTransform`) "Undefined" "MultiplyWithRoot" null null))
  (bind _output_get (set `self.EquippedWeapon` _returnvalue))
  (`self.SetOwner` _output_get self)
  (`self.K2_AttachToComponent` (`self.EquippedWeapon`) (`self.Mesh`) "Assault_Rifle_A_Socket" "SnapToTarget" "SnapToTarget" "SnapToTarget" true)
  (`self.Set Random Walk Speed`)
  (`BlackboardComponent.SetValueAsVector` (`self.BB`) "StartLocation" (`self.K2_GetActorLocation`))
  (`BlackboardComponent.SetValueAsVector` (`self.BB`) "PatrolLocation" (`SceneComponent.K2_GetComponentLocation` (`self.PatrolPoint`))))

(event `self.AIPerception.OnTargetPerceptionUpdated`
  (params (Actor :type "Actor Object Reference") (Stimulus :type "AIStimulus Structure"))
  (bind _bb (`self.BB`))
  (bind _asbp_third_person_character (cast `/Game/ThirdPerson/Blueprints/BP_ThirdPersonCharacter` Actor))
  (if Stimulus_bSuccessfullySensed
    (`BlackboardComponent.SetValueAsObject` _bb "Target" _asbp_third_person_character)
    (`BlackboardComponent.ClearValue` _bb "LastKnownLocation")
    (`SceneComponent.SetVisibility` (`self.AlertWidget`) true false)
    (set `self.targetSighted?` true)
    (set `self.targetLost?` false)
    (set `self.alarted!` true)
    (else
      (set `self.targetLost?` true)
      (`BlackboardComponent.SetValueAsVector` _bb "LastKnownLocation" Stimulus_StimulusLocation)
      (set `self.targetSighted?` false)))
  (set `self.AlertTimer` 0.0))

(event `self.ReceiveTick`
  (params (DeltaSeconds :type "Float (single-precision)"))
  (bind _bb (`self.BB`))
  (if (`self.targetLost?`)
    (bind _output_get (set `self.AlertTimer` (+ (`self.AlertTimer`) DeltaSeconds)))
    (if (> _output_get (`self.GiveUpTime`))
      (set `self.alarted!` false)
      (set `self.targetSighted?` false)
      (set `self.targetLost?` false)
      (`SceneComponent.SetVisibility` (`self.AlertWidget`) false false)
      (`BlackboardComponent.SetValueAsObject` _bb "Target" null)
      (`BlackboardComponent.ClearValue` _bb "LastKnownLocation"))))

(fn `HandleEnemyDeath`
  (`PrimitiveComponent.SetSimulatePhysics` (`self.Mesh`) true)
  (`PrimitiveComponent.SetCollisionEnabled` (`self.CapsuleComponent`) "NoCollision")
  (`self.SetActorEnableCollision` self false)
  (`self.DisableInput` (`AIBlueprintHelperLibrary.GetAIController` null) null))

(fn `Set Random Walk Speed`
  (set `self.Random Walk Speed` (`KismetMathLibrary.RandomFloatInRange` 75.0 200.0))
  (set `self.BB` (`AIBlueprintHelperLibrary.GetBlackboard` null))
  (`BlackboardComponent.SetValueAsFloat` (`self.BB`) "MaxWalkSpeed" (`self.Random Walk Speed`)))

(fn `UserConstructionScript`)