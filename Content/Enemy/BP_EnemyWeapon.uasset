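; BP_EnemyWeapon is an enemy hitscan weapon that fires at a given target actor when FireAtTarget is called.
; It plays a rifle sound and attaches a muzzle flash at the skeletal mesh's barrel socket.
; A Camera-channel line trace runs from the barrel to the target's location, ignoring the instigator pawn.
; Whatever actor it hits takes NPCDamage, credited to the instigator's controller.
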(fn `FireAtTarget`
  (params (TargetActor :type "Actor Object Reference") (InstigatorPawn :type "Pawn Object Reference"))
  (bind _skeletalmesh (`self.SkeletalMesh`))
  (bind _instigatorpawn (`local.InstigatorPawn`))
  (bind _returnvalue (`SceneComponent.GetSocketLocation` _skeletalmesh "barrel"))
  (`GameplayStatics.PlaySoundAtLocation` "/Game/MilitaryWeapSilver/Sound/Rifle/Wavs/RifleA_Fire01.RifleA_Fire01" _returnvalue (struct) 1.0 1.0 0.0 null null null null)
  (`GameplayStatics.SpawnEmitterAttached` "/Game/MilitaryWeapSilver/FX/P_AssaultRifle_MuzzleFlash.P_AssaultRifle_MuzzleFlash" _skeletalmesh "barrel")
  (bind (_outhit _returnvalue_2) (`KismetSystemLibrary.LineTraceSingle` _returnvalue (`self.K2_GetActorLocation` (`local.TargetActor`)) "TraceTypeQuery2" false (`|MakeArray` (`local.InstigatorPawn`) :!type "Actor Object Reference")))
  (if _returnvalue_2
    (`GameplayStatics.ApplyDamage` (`.HitActor` (`GameplayStatics.BreakHitResult` _outhit)) (`self.NPCDamage`) (`Pawn.GetController` _instigatorpawn) _instigatorpawn)
    (return)
    (else
      (return))))

(fn `UserConstructionScript`)